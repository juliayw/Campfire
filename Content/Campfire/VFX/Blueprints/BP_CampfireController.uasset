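; BP_CampfireController is a keyboard-driven test actor that switches a campfire VFX between a start and an end effect.
; BeginPlay enables input from player controller 0 on the actor.
; Pressing P deactivates CampfireEnd and sets CamfireStart active from the Start variable, while O does the reverse using the End variable, both without resetting.
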(event EventBeginPlay
  (Input|EnableInput (Game|GetPlayerController 0)))

(event Input|KeyboardEvents|P
  (params (Key :type Key%20Structure :default "None"))
  ;[1 1 1] Press"P" to trigger the campfire
  (:Pressed
    (Components|Activation|Deactivate (Variables|Default|GetCampfire_End))
    (Components|Activation|SetActive (Variables|Default|GetCamfire_Start) (Variables|Default|GetStart) false)))

(event Input|KeyboardEvents|O
  (params (Key :type Key%20Structure :default "None"))
  ;[1 1 1] Press “O” to deactive the campfire
  (:Pressed
    (Components|Activation|Deactivate (Variables|Default|GetCamfire_Start))
    (Components|Activation|SetActive (Variables|Default|GetCampfire_End) (Variables|Default|GetEnd) false)))

(fn ConstructionScript)